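; Player controller for LeaveMeAlone that opens the pause and end-game menus.
; Pause input, guarded by a flag, pauses the game, shows the pause widget with UI-only input and cursor, and stops the player's weapon fire; unpausing is not handled here.
; UnPossess, treated as player death, starts a short timer that pauses the game and shows the end-game widget.
; An older Delay-based version of the death menu remains disconnected.
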(event Custom|DeathEvent
  ;[1 1 1] Вызов меню, после смерти персонажа c помощью таймера
  (Utilities|Time|ClearandInvalidateTimerbyHandle (Variables|Default|GetdeathTimerHandler))
  (Game|SetGamePaused true)
  (bind _returnvalue (UserInterface|CreateWidget "/Game/LeaveMeAlone/Widgets/UI/WBP_EndGame.WBP_EndGame_C"))
  (bind _output_get (Variables|Default|SetEndGameWidget _returnvalue))
  (UserInterface|Viewport|AddtoViewport _output_get 0)
  (Input|SetInputModeUIOnly self _returnvalue "DoNotLock" false)
  (Variables|Default|SetbShowMouseCursor true))

(event EventBeginPlay)

(event EventTick
  (params (DeltaSeconds :type Float%20%28single-precision%29)))

(event EventUnPossess
  (params (UnpossessedPawn :type Pawn%20Object%20Reference))
  ;[1 1 1] Вызов меню, после смерти персонажа c помощью таймера
  (bind _returnvalue (Utilities|Time|SetTimerbyEvent (delegate Custom|DeathEvent) 3.0))
  (Variables|Default|SetdeathTimerHandler _returnvalue))

(event Input|ActionEvents|InputActionPause
  (params (Key :type Key%20Structure :default "None"))
  ;[1 1 1] Срабатывание нажатия паузы и вызов меню паузы игры
  (:Pressed
    (if (not (Variables|Default|GetOnPause))
      (Variables|Default|SetOnPause true)
      (Game|SetGamePaused true)
      (bind _returnvalue (UserInterface|CreateWidget "/Game/LeaveMeAlone/Widgets/UI/WBP_Pause.WBP_Pause_C"))
      (bind _output_get (Variables|Default|SetPauseWidget _returnvalue))
      (UserInterface|Viewport|AddtoViewport _output_get 0)
      (Input|SetInputModeUIOnly self _output_get "DoNotLock" false)
      (Variables|Default|SetbShowMouseCursor true)
      (if (Variables|Default|GetOnPause)
        (bind _asch_player (Utilities|Casting|CastToCH_Player (Game|GetPlayerCharacter 0)))
        (Class|LMAWeaponComponent|StopFire (Variables|/Script/LeaveMeAlone.LMADefaultCharacter|GetWeaponComponent _asch_player))))))

(fn ConstructionScript)